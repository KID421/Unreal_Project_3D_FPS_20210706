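; Zombie enemy character that wanders, chases the player on sight and melee-attacks within stopping distance.
; A delayed Tick picks random nearby reachable points until pawn sensing spots someone, then AIMoveTo pursues the player.
; On arrival it halts and enables attack-zone overlaps for a timed window to damage the player.
; Bullet overlaps reduce health, triggering pursuit and impact effects, or ragdoll death, a HUD monster-count increment and delayed destruction.
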(event OnSeePawn(當前感應器)
  (params (Pawn :type Pawn%20Object%20Reference))
  (bind _charactermovement (Variables|Character|GetCharacterMovement))
  (bind _攻擊碰撞區域 (Variables|Default|Get攻擊碰撞區域))
  ;[1 1 1] 追蹤玩家
  (Variables|Default|Set是否看到玩家 true)
  (AI|AIMoveTo self "0, 0, 0" (Variables|Default|Get玩家) (Variables|Default|Get停止距離) false
    (:OnSuccess
      ;[1 1 1] 攻擊
      (Variables|Default|Set是否攻擊 true)
      (Variables|/Script/Engine.CharacterMovementComponent|SetMaxWalkSpeed _charactermovement 0.0)
      (Variables|/Script/Engine.PrimitiveComponent|SetbGenerateOverlapEvents _攻擊碰撞區域 true)
      (Utilities|FlowControl|Delay 3.0)
      (Variables|Default|Set是否攻擊 false)
      (Variables|/Script/Engine.CharacterMovementComponent|SetMaxWalkSpeed _charactermovement 6e+02)
      (Variables|/Script/Engine.PrimitiveComponent|SetbGenerateOverlapEvents _攻擊碰撞區域 false))))

(event OnComponentBeginOverlap(攻擊碰撞區域)
  (params (OverlappedComponent :type Primitive%20Component%20Object%20Reference) (OtherActor :type Actor%20Object%20Reference) (OtherComp :type Primitive%20Component%20Object%20Reference) (OtherBodyIndex :type Integer) (bFromSweep :type Boolean) (SweepResult :type Hit%20Result%20Structure%20%28by%20ref%29))
  (bind _asbp_玩家控制 (Utilities|Casting|CastToBP_玩家控制 OtherActor))
  (Default|受傷 _asbp_玩家控制 (Variables|Default|Get攻擊力)))

(event EventBeginPlay
  ;[1 1 1] 取得玩家資訊
  (bind _asbp_玩家控制 (Utilities|Casting|CastToBP_玩家控制 (Game|GetPlayerCharacter 0)))
  (Variables|Default|Set玩家 _asbp_玩家控制))

(event EventTick
  (params (DeltaSeconds :type Float%20%28single-precision%29))
  ;[1 1 1] 隨機走動
  (Utilities|FlowControl|Delay 3.0)
  (if (not (Variables|Default|Get是否看到玩家))
    (AI|AIMoveTo self (.RandomLocation (AI|Navigation|GetRandomReachablePointinRadius (Transformation|GetActorLocation) 2.5e+02 0 0)) 0 (Variables|Default|Get停止距離) false)))

(event Collision|EventActorBeginOverlap
  (params (OtherActor :type Actor%20Object%20Reference))
  (bind _玩家 (Variables|Default|Get玩家))
  (bind _主要介面 (Variables|/Game/BP/BP_玩家控制.BP_玩家控制_C|Get主要介面 _玩家))
  ;[1 1 1] 受傷
  (bind _asbp_子彈 (Utilities|Casting|CastToBP_子彈 OtherActor))
  (Variables|Default|Set血量 (- (Variables|Default|Get血量) (Variables|/Game/BP/BP_子彈.BP_子彈_C|Get傷害值 _asbp_子彈)))
  (if (<= (- (Variables|Default|Get血量) (Variables|/Game/BP/BP_子彈.BP_子彈_C|Get傷害值 _asbp_子彈)) 0.0)
    (Physics|SetSimulatePhysics (Variables|Character|GetMesh) true)
    (Collision|SetCollisionEnabled (Variables|Collision|GetCapsuleComponent) "NoCollision")
    (Variables|/Game/BP/BP_介面.BP_介面_C|Set怪物數量 _主要介面 (+ (Variables|/Game/BP/BP_介面.BP_介面_C|Get怪物數量 _主要介面) 1))
    (Utilities|FlowControl|Delay 2.0)
    (Actor|DestroyActor)
    (else
      (AI|AIMoveTo self "0, 0, 0" (Variables|Default|Get玩家) (Variables|Default|Get停止距離) false
        (:then
          (Effects|SpawnEmitteratLocation "/Game/InfinityBladeEffects/Effects/FX_Monsters/FX_Monster_Ausar/P_AU_Shieldslam_Impact.P_AU_Shieldslam_Impact" (Transformation|GetActorLocation _asbp_子彈)))))))

(fn ConstructionScript)