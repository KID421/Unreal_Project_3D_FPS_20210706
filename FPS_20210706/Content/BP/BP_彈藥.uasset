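; BP_彈藥 is an ammo pickup that the player collects with the 檢道具 input action.
; Overlapping the 感應區域 trigger as BP_玩家控制 sets an in-range flag and shows the 提示文字 prompt, which Tick rotates toward the player; leaving reverses both.
; Pressing the input while in range calls 添加彈藥 on the player's 武器 with a fixed amount, destroying the pickup only if that call succeeds.
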(event OnComponentBeginOverlap(感應區域)
  (params (OverlappedComponent :type Primitive%20Component%20Object%20Reference) (OtherActor :type Actor%20Object%20Reference) (OtherComp :type Primitive%20Component%20Object%20Reference) (OtherBodyIndex :type Integer) (bFromSweep :type Boolean) (SweepResult :type Hit%20Result%20Structure%20%28by%20ref%29))
  (Utilities|Casting|CastToBP_玩家控制 OtherActor)
  (Variables|Default|Set玩家是否進入 true)
  (Rendering|SetVisibility (Variables|Default|Get提示文字) true false))

(event OnComponentEndOverlap(感應區域)
  (params (OverlappedComponent :type Primitive%20Component%20Object%20Reference) (OtherActor :type Actor%20Object%20Reference) (OtherComp :type Primitive%20Component%20Object%20Reference) (OtherBodyIndex :type Integer))
  (Utilities|Casting|CastToBP_玩家控制 OtherActor)
  (Variables|Default|Set玩家是否進入 false)
  (Rendering|SetVisibility (Variables|Default|Get提示文字) false false))

(event EventTick
  (params (DeltaSeconds :type Float%20%28single-precision%29))
  (bind _提示文字 (Variables|Default|Get提示文字))
  (if (Variables|Default|Get玩家是否進入)
    (Transformation|SetRelativeLocationAndRotation _提示文字 (Variables|/Script/Engine.SceneComponent|GetRelativeLocation _提示文字) (Math|Rotator|FindLookatRotation (Transformation|GetWorldLocation _提示文字) (Transformation|GetActorLocation (Game|GetPlayerCharacter 0))) false false)))

(event Input|ActionEvents|InputAction檢道具
  (params (Key :type Key%20Structure :default "None"))
  (:Pressed
    (if (Variables|Default|Get玩家是否進入)
      (bind _asbp_玩家控制 (Utilities|Casting|CastToBP_玩家控制 (Game|GetPlayerCharacter 0)))
      (bind _是否有補充彈藥 (Default|添加彈藥 (Variables|/Game/BP/BP_玩家控制.BP_玩家控制_C|Get武器 _asbp_玩家控制) 30))
      (if _是否有補充彈藥
        (Actor|DestroyActor)))))

(fn ConstructionScript)