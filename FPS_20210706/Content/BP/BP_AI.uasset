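; BP_AI is an enemy AI pawn that wanders, chases the player character and takes bullet damage.
; Tick uses a Delay to send it to random nearby reachable points until its sensor sees a pawn, then it moves toward the player.
; BP_子彈 overlaps reduce 血量, then destroy it if remaining health minus damage again is zero or less.
; Otherwise it chases the player and spawns an impact emitter.
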(event OnSeePawn(當前感應器)
  (params (Pawn :type Pawn%20Object%20Reference))
  (Variables|Default|Set是否看到玩家 true)
  (AI|AIMoveTo self "0, 0, 0" (Variables|Default|Get玩家) 5.0 false
    (:OnSuccess
      (Variables|Default|Set是否看到玩家 false))))

(event EventBeginPlay
  (bind _asbp_玩家控制 (Utilities|Casting|CastToBP_玩家控制 (Game|GetPlayerCharacter 0)))
  (Variables|Default|Set玩家 _asbp_玩家控制))

(event EventTick
  (params (DeltaSeconds :type Float%20%28single-precision%29))
  (Utilities|FlowControl|Delay 3.0)
  (if (not (Variables|Default|Get是否看到玩家))
    (AI|AIMoveTo self (.RandomLocation (AI|Navigation|GetRandomReachablePointinRadius (Transformation|GetActorLocation) 2.5e+02 0 0)) 0 5.0 false)))

(event Collision|EventActorBeginOverlap
  (params (OtherActor :type Actor%20Object%20Reference))
  ;[1 1 1] 受傷
  (bind _asbp_子彈 (Utilities|Casting|CastToBP_子彈 OtherActor))
  (Variables|Default|Set血量 (- (Variables|Default|Get血量) (Variables|/Game/BP/BP_子彈.BP_子彈_C|Get傷害值 _asbp_子彈)))
  (if (<= (- (Variables|Default|Get血量) (Variables|/Game/BP/BP_子彈.BP_子彈_C|Get傷害值 _asbp_子彈)) 0.0)
    (Actor|DestroyActor)
    (else
      (AI|AIMoveTo self "0,0.000000, 0" (Variables|Default|Get玩家) 5.0 false
        (:then
          (Effects|SpawnEmitteratLocation "/Game/InfinityBladeEffects/Effects/FX_Monsters/FX_Monster_Ausar/P_AU_Shieldslam_Impact.P_AU_Shieldslam_Impact" (Transformation|GetActorLocation _asbp_子彈)))))))

(fn ConstructionScript)