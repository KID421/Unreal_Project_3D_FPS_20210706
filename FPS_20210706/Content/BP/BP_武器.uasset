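; Weapon Blueprint that handles firing and magazine reloading with a limited ammo reserve.
; The 發射子彈 event uses up a round, then spawns a BP_子彈 bullet and a small muzzle-flash emitter at the weapon's 子彈插槽 socket.
; The 換彈匣 function tops up the magazine from the reserve, moving whatever remains when the reserve cannot fill it.
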(event Custom|發射子彈
  (bind _武器 (Variables|Default|Get武器))
  ;[1 1 1] 發射子彈
  (if (> (Variables|Default|Get子彈數量) 0)
    (Variables|Default|Set子彈數量 (- (Variables|Default|Get子彈數量) 1))
    (Game|SpawnActorfromClass "/Game/BP/BP_子彈.BP_子彈_C" (Transformation|GetSocketTransform _武器 "子彈插槽" "RTS_World") "Undefined" 0 0)
    (Effects|SpawnEmitteratLocation "/Game/InfinityBladeEffects/Effects/FX_Monsters/FX_Monster_Chicken/P_ChickenMaster_MuzzleFlash_01.P_ChickenMaster_MuzzleFlash_01" (Transformation|GetSocketLocation _武器 "子彈插槽") (Transformation|GetSocketRotation _武器 "子彈插槽") "0.100000,0.100000,0.100000")))

(fn ConstructionScript)

(fn 換彈匣
  (if (> (Variables|Default|Get子彈總數) 0) ; 總數大於零才能換
    (if (< (Variables|Default|Get子彈數量) (Variables|Default|Get彈匣尺寸)) ; 子彈數量小於彈匣才能換
      (if (>= (Variables|Default|Get子彈總數) (- (Variables|Default|Get彈匣尺寸) (Variables|Default|Get子彈數量))) ; 如果 子彈總數 >= 要補充的數量，先扣除要補充的數量\n否則 子彈總數 <   要補充的數量，就直接把總數加給子彈數
        (Variables|Default|Set子彈總數 (- (Variables|Default|Get子彈總數) (- (Variables|Default|Get彈匣尺寸) (Variables|Default|Get子彈數量))))
        (Variables|Default|Set子彈數量 (+ (Variables|Default|Get子彈數量) (- (Variables|Default|Get彈匣尺寸) (Variables|Default|Get子彈數量))))
        (else
          (Variables|Default|Set子彈數量 (+ (Variables|Default|Get子彈數量) (Variables|Default|Get子彈總數)))
          (Variables|Default|Set子彈總數 0))))))